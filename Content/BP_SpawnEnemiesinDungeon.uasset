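; Dungeon spawner actor that populates generated rooms with enemies and places the player.
; After a short delay on BeginPlay, it gathers the Scene component of every Dungeon_room_1 actor as unique spawn points.
; It spawns a random class from EnemyTypes at each point.
; It then spawns BP_Player at the last point, sharing it with an enemy, and calls Possess on the first player controller.
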(event EventBeginPlay
  (Utilities|FlowControl|Delay 2.0)
  (bind _outactors (Actor|GetAllActorsOfClass "/Game/Procedural/Dungeon_room_1.Dungeon_room_1_C"))
  (for _array_element _outactors
    (Utilities|Array|AddUnique (Variables|Default|GetSpawn%20Points) (Variables|/Game/Procedural/Master_room.Master_room_C|GetScene _array_element)))
  (for _array_element_2 (Variables|Default|GetSpawn%20Points)
    (Game|SpawnActorfromClass (.OutItem (Utilities|Array|Random (Variables|Default|GetEnemyTypes))) (Math|Transform|MakeTransform (Transformation|GetWorldLocation _array_element_2) "0, 0, 0" "1.000000,1.000000,1.000000") "Undefined" "MultiplyWithRoot" 0 2 0))
  (Development|PrintString "fp")
  (Game|SpawnActorfromClass "/Game/Player/BP_Player.BP_Player_C" (Math|Transform|MakeTransform (Transformation|GetWorldLocation _array_element_2) "0, 0, 0" "1.000000,1.000000,1.000000") "Undefined" "MultiplyWithRoot" 0 0)
  (Pawn|Possess (Game|GetPlayerController 0)))

(event Collision|EventActorBeginOverlap
  (params (OtherActor :type Actor%20Object%20Reference)))

(event EventTick
  (params (DeltaSeconds :type Float%20%28single-precision%29)))

(fn ConstructionScript)