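; BP_CompanionAI seeds the companion AI's Blackboard with the player and an enemy target when play begins.
; On BeginPlay it takes the first actor tagged "Player", casts it to BP_FirstPersonCharacter, caches it and writes it to the player key.
; It then writes a single Enemy_Base actor, found by class lookup, to the target key.
; The lookup runs once, with no later retargeting and no behavior tree started here.
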(event EventBeginPlay
  (bind _outactors (Actor|GetAllActorswithTag "Player"))
  (Utilities|IsValid (Utilities|Array|Get(acopy) _outactors)
    (:Is%20Valid
      (bind _asbp_first_person_character (Utilities|Casting|CastToBP_FirstPersonCharacter (Utilities|Array|Get(acopy) _outactors)))
      (bind _output_get (Variables|Default|SetPlayerRef _asbp_first_person_character))
      (AI|Components|Blackboard|SetValueasObject (AI|GetBlackboard 0) (Variables|Default|GetPlayerRefKey) _output_get)
      (bind _returnvalue (Actor|GetActorOfClass "/Game/EnemyAI/BP/Enemy_Base.Enemy_Base_C"))
      (Utilities|IsValid _returnvalue
        (:Is%20Valid
          (AI|Components|Blackboard|SetValueasObject (AI|GetBlackboard 0) (Variables|Default|GetTargetActorKey%20) _returnvalue))))))

(event Collision|EventActorBeginOverlap
  (params (OtherActor :type Actor%20Object%20Reference)))

(event EventTick
  (params (DeltaSeconds :type Float%20%28single-precision%29)))

(fn ConstructionScript)