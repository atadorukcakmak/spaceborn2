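; BP_Console is an actor that opens a screen interface when the first-person character enters its Box trigger.
; On overlap, it checks the other actor against the BP_FirstPersonCharacter found in the level, then creates a Screen_UI widget and adds it to the viewport.
; It also sets the player's movement mode to None, shows the mouse cursor and switches input to UI only.
; Nothing in this Blueprint restores movement or game input.
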(event OnComponentBeginOverlap(Box)
  (params (OverlappedComponent :type Primitive%20Component%20Object%20Reference) (OtherActor :type Actor%20Object%20Reference) (OtherComp :type Primitive%20Component%20Object%20Reference) (OtherBodyIndex :type Integer) (bFromSweep :type Boolean) (SweepResult :type Hit%20Result%20Structure%20%28by%20ref%29))
  (bind _returnvalue (Game|GetPlayerController 0))
  (bind _returnvalue_2 (Actor|GetActorOfClass "/Game/FirstPerson/Blueprints/BP_FirstPersonCharacter.BP_FirstPersonCharacter_C"))
  (if (== _returnvalue_2 OtherActor)
    (bind _returnvalue_3 (UserInterface|CreateWidget "/Game/Dilara/GameStart/Screen_UI.Screen_UI_C"))
    (UserInterface|Viewport|AddtoViewport _returnvalue_3 0)
    (Pawn|Components|CharacterMovement|SetMovementMode (Variables|/Script/Engine.Character|GetCharacterMovement (Game|GetPlayerCharacter 0)) "MOVE_None" 0)
    (Variables|/Script/Engine.PlayerController|SetbShowMouseCursor _returnvalue true)
    (Input|SetInputModeUIOnly _returnvalue 0 "DoNotLock" false)))

(event EventBeginPlay)

(event Collision|EventActorBeginOverlap
  (params (OtherActor :type Actor%20Object%20Reference)))

(event EventTick
  (params (DeltaSeconds :type Float%20%28single-precision%29)))

(fn ConstructionScript)