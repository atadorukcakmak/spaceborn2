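; BP_InteractPuzzle is an interactable that takes the player into a jigsaw puzzle.
; On interact, a timeline lerps the player's follow camera from its current transform to the actor's Scene location and a fixed yaw facing.
; When it finishes, it disables character movement, opens the JigsawWidget, shows the mouse cursor and zeroes the player's camera rotation multiplier.
; The file contains no logic to exit the puzzle or restore the camera.
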(event EventOnInteract
  (bind _bp_player (Variables|Default|GetBP_Player))
  (bind _bp_player_2 (Variables|Default|GetBP_Player))
  (bind _followcamera (Variables|/Game/Player/BP_Player.BP_Player_C|GetFollowCamera _bp_player))
  (bind _followcamera_2 (Variables|/Game/Player/BP_Player.BP_Player_C|GetFollowCamera _bp_player_2))
  (Variables|Default|SetInitialCameraLocation (Transformation|GetWorldLocation _followcamera_2))
  (Variables|Default|SetInitialCameraRotation (Transformation|GetWorldRotation _followcamera_2))
  (bind _cameralerp (Timeline|SetCamera PlayFromStart)
    (:Update
      (Transformation|SetWorldLocation _followcamera (Math|Vector|Lerp(Vector) (Variables|Default|GetInitialCameraLocation) (Transformation|GetWorldLocation (Variables|Default|GetScene)) _cameralerp) false false)
      (Transformation|SetWorldRotation _followcamera (Math|Rotator|Lerp(Rotator) (Variables|Default|GetInitialCameraRotation) "-90.000000,0.000000,0.000000" _cameralerp true) false false))
    (:Finished
      (Pawn|Components|CharacterMovement|SetMovementMode (Variables|/Script/Engine.Character|GetCharacterMovement (Game|GetPlayerCharacter 0)) "MOVE_None" 0)
      (bind _returnvalue (UserInterface|CreateWidget "/Game/Dilara/Puzzle/JigsawWidget.JigsawWidget_C"))
      (UserInterface|Viewport|AddtoViewport _returnvalue 0)
      (Variables|/Script/Engine.PlayerController|SetbShowMouseCursor (Game|GetPlayerController 0) true)
      (Variables|/Game/Player/BP_Player.BP_Player_C|SetCameraRotationMultiplier (Variables|Default|GetBP_Player) 0.0))))

(event EventBeginPlay
  (bind _returnvalue (Actor|GetActorOfClass "/Game/Player/BP_Player.BP_Player_C"))
  (Variables|Default|SetBP_Player _returnvalue))

(fn ConstructionScript)