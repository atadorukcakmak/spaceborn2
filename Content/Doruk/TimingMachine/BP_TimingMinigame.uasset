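; Timing-bar minigame machine where stopping a moving bar inside a random window gains or loses embryos, though its event-graph logic is currently disconnected from the empty events.
; CreateNewRound randomizes the window and passes it to a new WBP_Timing widget.
; Unwired chains lock movement, blend to TimingCamera, score five progressively faster rounds through MainGameInstance, then restore the player.
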(event Custom|PlayTimeEvent)

(event Collision|EventActorBeginOverlap
  (params (OtherActor :type Actor%20Object%20Reference)))

(event EventOnInteract)

(event EventBeginPlay)

(fn ConstructionScript)

(fn SetIntervalPoints
  (bind _output_get (Variables|IntervalPoints|SetClickableIntervalLength (Math|Random|RandomFloatinRange 0.12 0.3)))
  (bind _output_get_2 (Variables|IntervalPoints|SetInterval1 (Math|Random|RandomFloatinRange 0.0 0.87)))
  (if (< _output_get_2 (- 1.0 _output_get))
    (Variables|IntervalPoints|SetInterval2 (+ (Variables|IntervalPoints|GetInterval1) (Variables|IntervalPoints|GetClickableIntervalLength)))
    (Development|PrintString (Utilities|String|Append "Interval1: " (Utilities|String|ToString(Float) (Variables|IntervalPoints|GetInterval1)) "         " "Interval2: " (Utilities|String|ToString(Float) (Variables|IntervalPoints|GetInterval2)) "           " "Clickable Interval Length" (Utilities|String|ToString(Float) (Variables|IntervalPoints|GetClickableIntervalLength))) true true "(R=1.000000,G=0.934148,B=0.000000,A=1.000000)" 5e+01)
    (else
      (Variables|IntervalPoints|SetInterval2 1.0))))

(fn CreateWidget
  (bind _returnvalue (UserInterface|CreateWidget "/Game/Doruk/TimingMachine/WBP_Timing.WBP_Timing_C"))
  (bind _output_get (Variables|Default|SetWBP_Timing _returnvalue))
  (Variables|/Game/Doruk/TimingMachine/WBP_Timing.WBP_Timing_C|SetClickableIntervalLength _output_get (Variables|IntervalPoints|GetClickableIntervalLength))
  (Variables|/Game/Doruk/TimingMachine/WBP_Timing.WBP_Timing_C|SetInterval1 _output_get (Variables|IntervalPoints|GetInterval1))
  (Variables|/Game/Doruk/TimingMachine/WBP_Timing.WBP_Timing_C|SetInterval2 _output_get (Variables|IntervalPoints|GetInterval2))
  (UserInterface|Viewport|AddtoViewport _output_get 0))

(fn CreateNewRound
  (CallFunction|SetIntervalPoints)
  (CallFunction|CreateWidget))