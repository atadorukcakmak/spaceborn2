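; Ranged enemy Blueprint that attacks with a rifle montage and extends a parent enemy class.
; Attack plays the montage, then on completion or interruption signals attack end and sends fixed damage directly to the AI controller's AttackTarget, with no active hit trace.
; It supplies attack and defend ranges, while TakeDamage and IsDead always return false.
; EnterCover is empty, and crouch and line-trace nodes are unconnected.
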(event Custom|EnterCover)

(event EventBeginPlay
  (|CallParentFunction))

(event EventAttack
  (bind _notifyname (Animation|Montage|PlayMontage (Variables|Character|GetMesh) "/Game/AnimStarterPack/Fire_Rifle_Ironsights_Montage.Fire_Rifle_Ironsights_Montage")
    (:OnCompleted
      (Default|CallOnAttackEnd :!label _label)
      (bind _asai_controller (Utilities|Casting|CastToAI_Controller (AI|GetAIController self)))
      (Utilities|IsValid (Variables|/Game/EnemyAI/AI_Controller.AI_Controller_C|GetAttack%20Target _asai_controller)
        (:Is%20Valid
          (Class|BPIDamagable|TakeDamage(Message) (Variables|/Game/EnemyAI/AI_Controller.AI_Controller_C|GetAttack%20Target _asai_controller) (Utilities|Struct|MakeS_DamageInfo 3e+01 "NewEnumerator2" "NewEnumerator1")))))
    (:OnInterrupted
      (goto _label))
    (:OnNotifyBegin
      (switch name _notifyname))))

(fn ConstructionScript
  (|CallParentFunction))

(fn TakeDamage
  (params (DamageInfo :type S%20Damage%20Info%20Structure))
  (return false))

(fn IsDead
  (return false))

(fn GetIdealRange
  (return 5e+02 2e+02))