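; BP_SaveHostage is a rescue point that spawns hostages and, when interacted with, frees them to join the player's team.
; On BeginPlay it spawns HostageNumber BP_Hostage actors at its Sphere's location, adjusting for collisions, and caches the player as BP_Player.
; OnInteract calls BreakFree on each stored hostage, adds it to the player's MyTeam array, then destroys the rescue actor.
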(event EventBeginPlay
  (CallFunction|SpawnHostages (Variables|Default|GetHostage%20Number))
  (bind _asbp_player (Utilities|Casting|CastToBP_Player (Game|GetPlayerCharacter 0)))
  (Variables|Default|SetAs%20BP%20Player _asbp_player))

(event EventOnInteract
  (for _array_element (Variables|Default|GetHostageArr)
    (Default|BreakFree _array_element)
    (CallFunction|AddMyTeam _array_element))
  (Actor|DestroyActor))

(fn ConstructionScript)

(fn SpawnHostages
  (params (Hostage%20Number :type Integer))
  (for _index (range 1 Hostage%20Number)
    (bind _returnvalue (Game|SpawnActorfromClass "/Game/Enemies/MageEnemy/BP_Hostage.BP_Hostage_C" (Math|Transform|MakeTransform (Transformation|GetWorldLocation (Variables|Default|GetSphere)) "0, 0, 0" "1.000000,1.000000,1.000000") "AdjustIfPossibleButAlwaysSpawn" "MultiplyWithRoot" 0 99 0))
    (Utilities|Array|Add (Variables|Default|GetHostageArr) _returnvalue)))

(fn AddMyTeam
  (params (NewItem :type BP%20Enemy%20Base%20Object%20Reference%20%28by%20ref%29))
  (Utilities|Array|Add (Variables|/Game/Player/BP_Player.BP_Player_C|GetMyTeam (Variables|Default|GetAs%20BP%20Player)) NewItem))