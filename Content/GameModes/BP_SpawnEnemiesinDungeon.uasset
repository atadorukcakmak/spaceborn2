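; Dungeon population actor that places a steal object, enemies and the player at random room spawn points.
; After a short BeginPlay delay, it gathers Scene components from five dungeon room classes, then spawns BP_StealObject and relocates the existing player with fixed offsets.
; The GameInstance's active level sets the count of random enemy types.
; Each enemy spawn removes a separately randomized point, so locations can repeat.
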(event Custom|CustomDelay
  (Utilities|FlowControl|Delay 3.0))

(event EventBeginPlay
  (bind _asmy_game_instance (Utilities|Casting|CastToMyGameInstance (Game|GetGameInstance)))
  (Variables|Default|SetGameInstance _asmy_game_instance)
  (Utilities|FlowControl|Delay 2.0)
  (bind _returnvalue (Actor|GetActorOfClass "/Game/Player/BP_Player.BP_Player_C"))
  (Variables|Default|Setplayer _returnvalue)
  (CallFunction|CollectAllScenes))

(event Collision|EventActorBeginOverlap
  (params (OtherActor :type Actor%20Object%20Reference)))

(event EventTick
  (params (DeltaSeconds :type Float%20%28single-precision%29)))

(fn ConstructionScript)

(fn CollectAllScenes
  (bind _outactors (Actor|GetAllActorsOfClass "/Game/Procedural/Dungeon_room_1.Dungeon_room_1_C"))
  (for _array_element _outactors
    (Utilities|Array|AddUnique (Variables|Default|GetSpawn%20Points) (Variables|/Game/Procedural/Master_room.Master_room_C|GetScene _array_element)))
  (bind _outactors_2 (Actor|GetAllActorsOfClass "/Game/Procedural/Dungeon_room_left.Dungeon_room_left_C"))
  (for _array_element_2 _outactors_2
    (Utilities|Array|AddUnique (Variables|Default|GetSpawn%20Points) (Variables|/Game/Procedural/Master_room.Master_room_C|GetScene _array_element_2)))
  (bind _outactors_3 (Actor|GetAllActorsOfClass "/Game/Procedural/Dungeon_room_right.Dungeon_room_right_C"))
  (for _array_element_3 _outactors_3
    (Utilities|Array|AddUnique (Variables|Default|GetSpawn%20Points) (Variables|/Game/Procedural/Master_room.Master_room_C|GetScene _array_element_3)))
  (bind _outactors_4 (Actor|GetAllActorsOfClass "/Game/Procedural/Dungeon_room_stairs.Dungeon_room_stairs_C"))
  (for _array_element_4 _outactors_4
    (Utilities|Array|AddUnique (Variables|Default|GetSpawn%20Points) (Variables|/Game/Procedural/Master_room.Master_room_C|GetScene _array_element_4)))
  (bind _outactors_5 (Actor|GetAllActorsOfClass "/Game/Procedural/Dungeon_room_straight.Dungeon_room_straight_C"))
  (for _array_element_5 _outactors_5
    (Utilities|Array|AddUnique (Variables|Default|GetSpawn%20Points) (Variables|/Game/Procedural/Master_room.Master_room_C|GetScene _array_element_5)))
  (Game|SpawnActorfromClass "/Game/drk/Blueprints/BP_StealObject.BP_StealObject_C" (Math|Transform|MakeTransform (+ (Transformation|GetWorldLocation (.OutItem (Utilities|Array|Random (Variables|Default|GetSpawn%20Points)))) "175.000000,25.000000,0.000000") "0, 0, 0" "1.000000,1.000000,1.000000") "Undefined" "MultiplyWithRoot" 0 0)
  (CallFunction|DecideLeveltoSpawnEnemies)
  (Transformation|SetActorLocation (Variables|Default|Getplayer) (+ (Transformation|GetWorldLocation (.OutItem (Utilities|Array|Random (Variables|Default|GetSpawn%20Points)))) "-250.000000,150.000000,0.000000") false false)
  (Development|PrintString "Hello" true true "(R=0.301258,G=1.000000,B=0.000000,A=1.000000)"))

(fn DecideLeveltoSpawnEnemies
  (if (== (Variables|/Game/FirstPerson/Blueprints/MyGameInstance.MyGameInstance_C|GetActiveLevel (Variables|Default|GetGameInstance)) 1)
    (CallFunction|SpawnEnemies 4)
    (elif (== (Variables|/Game/FirstPerson/Blueprints/MyGameInstance.MyGameInstance_C|GetActiveLevel (Variables|Default|GetGameInstance)) 2)
      (CallFunction|SpawnEnemies 7)
      (elif (== (Variables|/Game/FirstPerson/Blueprints/MyGameInstance.MyGameInstance_C|GetActiveLevel (Variables|Default|GetGameInstance)) 3)
        (CallFunction|SpawnEnemies 9)
        (elif (== (Variables|/Game/FirstPerson/Blueprints/MyGameInstance.MyGameInstance_C|GetActiveLevel (Variables|Default|GetGameInstance)) 4)
          (CallFunction|SpawnEnemies 11)
          (else
            (CallFunction|SpawnEnemies 13)))))))

(fn SpawnEnemies
  (params (NumOfEnemies :type Integer))
  (bind _spawn_points (Variables|Default|GetSpawn%20Points))
  (bind _outitem (Utilities|Array|Random _spawn_points))
  (for _index (range 0 (- NumOfEnemies 1))
    (Game|SpawnActorfromClass (.OutItem (Utilities|Array|Random (Variables|Default|GetEnemyTypes))) (Math|Transform|MakeTransform (Transformation|GetWorldLocation _outitem) "0, 0, 0" "1.000000,1.000000,1.000000") "Undefined" "MultiplyWithRoot" 0 2 0)
    (Utilities|Array|RemoveItem (Variables|Default|GetSpawn%20Points) _outitem)))

(fn SpawnCharacter
  (Game|SpawnActorfromClass "/Game/Player/BP_Player.BP_Player_C" (Math|Transform|MakeTransform (Transformation|GetWorldLocation (.OutItem (Utilities|Array|Random (Variables|Default|GetSpawn%20Points)))) "0, 0, 0" "1.000000,1.000000,1.000000") "Undefined" "MultiplyWithRoot" 0 0)
  (Pawn|Possess (Game|GetPlayerController 0)))