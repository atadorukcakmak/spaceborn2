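; BP_world is a procedural terrain Blueprint meant to build a grid mesh with heights from 2D FastNoise.
; SetupFastNoise calls CreateVertices and CreateTriangles, then feeds vertices, indices and UVs into a procedural mesh section and applies a material.
; It is unfinished: BeginPlay and construction are empty, nothing here calls SetupFastNoise, the noise settings are unused, and the vertex-generation loop is disconnected, leaving only triangle indices generated.
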(event EventBeginPlay)

(fn ConstructionScript)

(fn CreateVertices)

(fn CreateTriangles
  (for _index (range 0 (- (Variables|Default|GetXSize) 1))
    (for _index_2 (range 0 (- (Variables|Default|GetYSize) 1))
      (Utilities|Array|Add (Variables|Default|GetTriangles) (LocalVariables|GetVertex))
      (Utilities|Array|Add (Variables|Default|GetTriangles) (+ (LocalVariables|GetVertex) 1))
      (Utilities|Array|Add (Variables|Default|GetTriangles) (+ (Variables|Default|GetYSize) (LocalVariables|GetVertex) 1))
      (Utilities|Array|Add (Variables|Default|GetTriangles) (+ (LocalVariables|GetVertex) 1))
      (Utilities|Array|Add (Variables|Default|GetTriangles) (+ (Variables|Default|GetYSize) 2 (LocalVariables|GetVertex)))
      (Utilities|Array|Add (Variables|Default|GetTriangles) (+ (Variables|Default|GetYSize) (LocalVariables|GetVertex) 1))
      (Math|Integer|IncrementInt (LocalVariables|GetVertex)))
    (Math|Integer|IncrementInt (LocalVariables|GetVertex))))